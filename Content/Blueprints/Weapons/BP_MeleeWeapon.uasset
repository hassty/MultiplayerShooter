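; Melee weapon Blueprint that deals point damage to whatever a short sphere trace hits in front of the player.
; AbleToUseWeapon reports readiness while no valid cooldown timer handle exists.
; When the parent UseWeapon succeeds, the server traces from the player camera along the owner's forward vector, applies damage and calls OnWeaponDamagedActor.
; Remote instances only play weapon effects.
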(fn `AbleToUseWeapon`
  (returns (Out :type Boolean))
  (return (not (`KismetSystemLibrary.K2_IsValidTimerHandle` (`self.CooldownTimer`)))))

(fn `GetOverlapInfo`
  (returns (Hit :type "HitResult Structure"))
  (bind _asbp_player_character (cast `/Game/Blueprints/Player/BP_PlayerCharacter` (`self.GetInstigator`))
    (:`then`
      (bind _returnvalue (`SceneComponent.K2_GetComponentLocation` (`/Game/Blueprints/Player/BP_PlayerCharacter.Camera` _asbp_player_character)))
      (bind _outhit (`KismetSystemLibrary.SphereTraceSingleForObjects` _returnvalue (+ _returnvalue (* (`self.GetActorForwardVector` (`self.GetOwner`)) (`self.Radius`))) 30.0 (`|MakeArray` "ObjectTypeQuery1" "ObjectTypeQuery2" "ObjectTypeQuery3" :!type "EObjectTypeQuery Enum") false (`|MakeArray` (`self.GetInstigator`) self :!type "Actor Object Reference")))
      (return _outhit))
    (:`CastFailed`
      (return))))

(fn `UserConstructionScript`
  (`parent.UserConstructionScript`))

(fn `UseWeapon`
  (returns (Used :type Boolean))
  (bind _used (`parent.UseWeapon`))
  (if _used
    (`/Engine/EditorBlueprintResources/ActorMacros.Switch Has Authority`
      (:`Authority`
        (bind _hit (`self.GetOverlapInfo`))
        (bind (_bblockinghit _binitialoverlap _time _distance _location _impactpoint _normal _impactnormal _physmat _hitactor _hitcomponent _hitbonename _hititem _faceindex _tracestart _traceend) (`GameplayStatics.BreakHitResult` _hit))
        (bind _returnvalue (`GameplayStatics.ApplyPointDamage` _hitactor (`self.Damage`) (`KismetMathLibrary.GetDirectionUnitVector` _traceend _tracestart) _hit (`self.GetInstigatorController`) self))
        (`self.OnWeaponDamagedActor` _returnvalue _hitactor)
        (return true))
      (:`Remote`
        (`self.PlayWeaponEffects`)))
    (else
      (return false))))