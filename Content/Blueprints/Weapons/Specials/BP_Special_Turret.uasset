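; Networked special-weapon turret that automatically fires on living enemy player characters within its radius, sparing its instigator and, in team modes, teammates.
; The server picks targets through radius overlaps, binds to their death, retargets when they leave, and applies line-trace point damage on a looping timer.
; Clients drop the radius component, follow the replicated Target via OnRep to run their own timer, and handle only platform aiming and muzzle flashes.
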(event `self.ReceiveTick`
  (params (DeltaSeconds :type "Float (single-precision)"))
  (`parent.ReceiveTick` DeltaSeconds)
  (`/Engine/EditorBlueprintResources/ActorMacros.Switch Has Authority`
    (:`Remote`
      (bind _target (`self.Target`)
        (:`then`
          (bind (_returnvalue_roll _returnvalue_pitch _returnvalue_yaw) (`KismetMathLibrary.BreakRotator` (`KismetMathLibrary.FindLookAtRotation` (`SceneComponent.K2_GetComponentLocation` (`self.PitchPlatform`)) (`self.K2_GetActorLocation` _target))))
          (`SceneComponent.K2_SetWorldRotation` (`self.YawPlatform`) (`KismetMathLibrary.MakeRotator` 0.0 0.0 _returnvalue_yaw) false false)
          (`SceneComponent.K2_SetRelativeRotation` (`self.PitchPlatform`) (`KismetMathLibrary.MakeRotator` 0.0 _returnvalue_pitch) false false))
        (:`else`)))))

(event `self.ReceiveBeginPlay`
  (`parent.ReceiveBeginPlay`)
  (`/Engine/EditorBlueprintResources/ActorMacros.Switch Has Authority`
    (:`Remote`
      (`ActorComponent.K2_DestroyComponent` (`self.TurretRadius`)))))

(event `self.TurretRadius.OnComponentBeginOverlap`
  (params (OverlappedComponent :type "PrimitiveComponent Object Reference") (OtherActor :type "Actor Object Reference") (OtherComp :type "PrimitiveComponent Object Reference") (OtherBodyIndex :type Integer) (bFromSweep :type Boolean) (SweepResult :type "HitResult Structure (by ref)"))
  (bind _asbp_player_character (cast `/Game/Blueprints/Player/BP_PlayerCharacter` OtherActor))
  (`self.Target`
    (:`then`)
    (:`else`
      (`self.SetTarget` _asbp_player_character))))

(event `self.TurretRadius.OnComponentEndOverlap`
  (params (OverlappedComponent :type "PrimitiveComponent Object Reference") (OtherActor :type "Actor Object Reference") (OtherComp :type "PrimitiveComponent Object Reference") (OtherBodyIndex :type Integer))
  (if (== OtherActor (`self.Target`))
    (`self.ClearTarget`)))

(event `self.ReceiveDestroyed`
  (`KismetSystemLibrary.K2_ClearAndInvalidateTimerHandle` (`self.ShootTimer`)))

(fn `ClearTarget`
  (set `self.Target` null)
  (`self.StopShoot`)
  (`self.FindNewTarget`))

(fn `FindNewTarget`
  (for _array_element (`PrimitiveComponent.GetOverlappingActors` (`self.TurretRadius`) "/Game/Blueprints/Player/BP_PlayerCharacter.BP_PlayerCharacter_C")
    (bind _asbp_player_character (cast `/Game/Blueprints/Player/BP_PlayerCharacter` _array_element :!pure true))
    (if (`self.ShouldAlarmOnCharacter` _asbp_player_character)
      (set `self.Target` _asbp_player_character)
      (`self.StartShoot`)
      (return))))

(fn `OnRep_Target`
  (`self.Target`
    (:`then`
      (`self.StartShoot`))
    (:`else`
      (`self.StopShoot`))))

(fn `SetTarget`
  (params (Target :type "/Game/Blueprints/Player/BP_PlayerCharacter Object Reference"))
  (locals (L_Target :type "/Game/Blueprints/Player/BP_PlayerCharacter Object Reference"))
  (bind _output_get (set `local.L_Target` Target))
  (if (`self.ShouldAlarmOnCharacter` _output_get)
    (set `self.Target` (`local.L_Target`))
    (`self.StartShoot`)
    (add `/Game/Blueprints/Components/Player/BP_HealthComponent.CharDead` (`/Game/Blueprints/Player/BP_PlayerCharacter.BP_HealthComponent` (`self.Target`)) (`|CreateDelegate` :!event `ClearTarget`))))

(fn `Shoot`
  (`self.Target`
    (:`then`
      (`/Engine/EditorBlueprintResources/ActorMacros.Switch Has Authority`
        (:`Authority`
          (bind _outhit (`KismetSystemLibrary.LineTraceSingleForObjects` (`SceneComponent.K2_GetComponentLocation` (`self.PitchPlatform`)) (`self.K2_GetActorLocation` (`self.Target`)) (`|MakeArray` "ObjectTypeQuery1" "ObjectTypeQuery2" "ObjectTypeQuery3" :!type "EObjectTypeQuery Enum")))
          (bind (_bblockinghit _binitialoverlap _time _distance _location _impactpoint _normal _impactnormal _physmat _hitactor _hitcomponent _hitbonename _hititem _faceindex _tracestart) (`GameplayStatics.BreakHitResult` _outhit))
          (if _bblockinghit
            (`GameplayStatics.ApplyPointDamage` _hitactor (`self.Damage`) (`KismetMathLibrary.GetDirectionUnitVector` _location _tracestart) _outhit (`self.GetInstigatorController`) self)))
        (:`Remote`
          (`GameplayStatics.SpawnEmitterAttached` "/Game/Assets/StarterContent/Particles/P_GunFlash.P_GunFlash" (`self.Turret1`) "None" (0.0 0.0 50.0) (struct) (5.0 5.0 5.0))
          (`GameplayStatics.SpawnEmitterAttached` "/Game/Assets/StarterContent/Particles/P_GunFlash.P_GunFlash" (`self.Turret2`) "None" (0.0 0.0 50.0) (struct) (5.0 5.0 5.0)))))
    (:`else`
      (`self.StopShoot`))))

(fn `ShouldAlarmOnCharacter`
  (params (Character :type "/Game/Blueprints/Player/BP_PlayerCharacter Object Reference"))
  (returns (Out :type Boolean))
  (if (not (`/Game/Blueprints/Components/Player/BP_HealthComponent.Dead` (`/Game/Blueprints/Player/BP_PlayerCharacter.BP_HealthComponent` Character)))
    (bind _instigator (`self.Instigator`)
      (:`then`
        (if (== _instigator Character)
          (return false)
          (else
            (`/Engine/EditorBlueprintResources/StandardMacros.IsValid` (`/Game/Blueprints/Libs/Functions/BP_Functions_GlobalGetters.GetTeamGameMode`)
              (:`Is Valid`
                (return (`/Game/Blueprints/Libs/Functions/BP_Functions_GlobalGetters.IsAnotherTeam` (`self.GetInstigatorController`) (`Pawn.GetController` Character))))
              (:`Is Not Valid`
                (return true))))))
      (:`else`
        (return true)))))

(fn `StartShoot`
  (bind _returnvalue (`KismetSystemLibrary.K2_SetTimer` null "Shoot" (`self.ShootDelay`) true))
  (set `self.ShootTimer` _returnvalue))

(fn `StopShoot`
  (`KismetSystemLibrary.K2_ClearAndInvalidateTimerHandle` (`self.ShootTimer`)))

(fn `UserConstructionScript`
  (`parent.UserConstructionScript`))