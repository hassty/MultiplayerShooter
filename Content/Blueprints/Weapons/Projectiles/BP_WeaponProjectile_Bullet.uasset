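; Bullet weapon projectile that deals point damage and leaves a bullet hole when it hits.
; On authority, the hit applies damage, reports the result to the owning Weapon and destroys the projectile.
; On remote, it spawns a short-lived decal actor aligned to the hit normal, using the hole material from BP_FireWeapons, so the impact visual is created locally rather than replicated.
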(event `self.ReceiveHit`
  (params (MyComp :type "PrimitiveComponent Object Reference") (Other :type "Actor Object Reference") (OtherComp :type "PrimitiveComponent Object Reference") (bSelfMoved :type Boolean) (HitLocation :type "Vector Structure") (HitNormal :type "Vector Structure") (NormalImpulse :type "Vector Structure") (Hit :type "HitResult Structure (by ref)"))
  (bind (_bblockinghit _binitialoverlap _time _distance _location _impactpoint _normal _impactnormal _physmat _hitactor _hitcomponent _hitbonename _hititem _faceindex _tracestart _traceend) (`GameplayStatics.BreakHitResult` Hit))
  (`/Engine/EditorBlueprintResources/ActorMacros.Switch Has Authority`
    (:`Authority`
      (bind _returnvalue (`GameplayStatics.ApplyPointDamage` Other (`self.Damage`) (`KismetMathLibrary.GetDirectionUnitVector` _traceend _tracestart) Hit (`self.GetInstigatorController`) (`self.GetOwner`)))
      (`/Game/Blueprints/Weapons/BP_Weapon.OnWeaponDamagedActor` (`self.Weapon`) _returnvalue Other)
      (`self.K2_DestroyActor`))
    (:`Remote`
      (bind _returnvalue_2 (`|SpawnActorFromClass` "/Script/Engine.DecalActor" (`KismetMathLibrary.MakeTransform` _location (struct) (0.01 0.01 0.01)) "AlwaysSpawn" "OverrideRootScale" null null))
      (`self.SetLifeSpan` _returnvalue_2 10.0)
      (`self.K2_SetActorRotation` _returnvalue_2 (`KismetMathLibrary.Conv_VectorToRotator` _normal) false)
      (bind _decal (`DecalActor.Decal` _returnvalue_2))
      (`DecalComponent.SetDecalMaterial` _decal (`/Game/Blueprints/Weapons/BP_FireWeapons.HoleMaterial` (cast `/Game/Blueprints/Weapons/BP_FireWeapons` (`self.Weapon`) :!pure true)))
      (`DecalComponent.SetFadeScreenSize` _decal 1e-05))))

(fn `UserConstructionScript`
  (`parent.UserConstructionScript`))