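; Shotgun weapon Blueprint that fires multiple pellets per shot by extending a parent weapon class.
; It overrides both the trace and projectile fire events, calling the parent version once for each count in ShotgunSpreadTraces.
; Visual fire effects take their world transform from the Skt_GunFire socket on the static mesh.
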(event `self.ShootFireTrace`
  (for _ (range 1 (+ (`self.ShotgunSpreadTraces`) 1))
    (`parent.ShootFireTrace`)))

(event `self.SpawnShootProjectile`
  (for _ (range 1 (+ (`self.ShotgunSpreadTraces`) 1))
    (`parent.SpawnShootProjectile`)))

(fn `UserConstructionScript`
  (`parent.UserConstructionScript`))

(fn `VisualFireTransform`
  (returns (Out :type "Transform Structure"))
  (return (`SceneComponent.GetSocketTransform` (`self.StaticMesh`) "Skt_GunFire" "RTS_World")))