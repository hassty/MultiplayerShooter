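; Sniper rifle weapon Blueprint that adds a scope overlay to the shared weapon behavior.
; ChangeScope runs the parent logic, then shows a lazily created, cached W_Scope widget on the viewport when scoping in and removes it when scoping out.
; VisualFireTransform supplies the world-space muzzle transform from the Skt_GunFire socket on the skeletal mesh.
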(event `self.ChangeScope`
  (params (Use :type Boolean))
  (`parent.ChangeScope` Use)
  (if Use
    (`self.SniperScope`
      (:`then`
        _)
      (:`else`
        (bind _returnvalue (`|CreateWidget` "/Game/UI/Other/Scope_Sniper/W_Scope.W_Scope_C"))
        (bind _output_get (set `self.SniperScope` _returnvalue))))
    (`UserWidget.AddToViewport` _output_get -1)
    (else
      (`Widget.RemoveFromParent` (`self.SniperScope`)))))

(fn `UserConstructionScript`
  (`parent.UserConstructionScript`))

(fn `VisualFireTransform`
  (returns (Out :type "Transform Structure"))
  (return (`SceneComponent.GetSocketTransform` (`self.SkeletalMesh_0`) "Skt_GunFire" "RTS_World")))