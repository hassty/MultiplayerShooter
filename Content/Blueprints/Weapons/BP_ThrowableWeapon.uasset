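; Throwable weapon Blueprint that launches a projectile, such as a grenade, when used by the player.
; UseWeapon runs the parent's use check, then calls ThrowGrenade only on the authority.
; ThrowGrenade spawns the projectile at the player camera, nudged along the owner's forward vector with a fixed angle offset, passing damage, weapon and instigator.
; When ammo is depleted, the owner's weapon manager drops the weapon.
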(fn `ThrowGrenade`
  (bind _asbp_player_character (cast `/Game/Blueprints/Player/BP_PlayerCharacter` (`self.GetInstigator`)))
  (`|SpawnActorFromClass` (`self.Projectile`) (`KismetMathLibrary.MakeTransform` (+ (`SceneComponent.K2_GetComponentLocation` (`/Game/Blueprints/Player/BP_PlayerCharacter.Camera` _asbp_player_character)) (* (`self.GetActorForwardVector` (`self.GetOwner`)) 70.0)) (`KismetMathLibrary.ComposeRotators` (`KismetMathLibrary.Conv_VectorToRotator` (`self.GetActorForwardVector` (`self.GetOwner`))) (struct :`Pitch` 10.0))) "Undefined" "OverrideRootScale" self (`self.Damage`) self (`self.GetInstigator`))
  (if (<= (`self.CurrentAmmo`) 0)
    (`/Game/Blueprints/Components/Player/BP_WeaponManager.DropWeapon` (`/Game/Blueprints/Player/BP_PlayerCharacter.BP_WeaponManager` (`self.WeaponOwner`)) self)))

(fn `UserConstructionScript`
  (`parent.UserConstructionScript`))

(fn `UseWeapon`
  (returns (Used :type Boolean))
  (bind _used (`parent.UseWeapon`))
  (if _used
    (`/Engine/EditorBlueprintResources/ActorMacros.Switch Has Authority`
      (:`Authority`
        (`self.ThrowGrenade`)
        (return true)))
    (else
      (return false))))