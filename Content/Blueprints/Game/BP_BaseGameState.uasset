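; Base game state that runs the round lifecycle on the server, from pre-start countdown through timed play to map vote and travel.
; A one-second authority tick counts down once enough players join, starts the round via the game mode, then reports time-limit expiry.
; Round end from the game mode is multicast, then BPMapVoteController's winner drives a ServerTravel.
; Dispatchers announce player connections and round start/end, with start fired from a RepNotify.
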(event `OnRoundEnded`
  (params (Reason :type String))
  (`self.Multicast-RoundEnd` Reason)
  (set `self.RoundInProgress` "NewEnumerator2")
  (`/Game/Blueprints/Components/Game/BP_MapVoteController.StartVote` (`self.BP_MapVoteController`))
  (add `/Game/Blueprints/Components/Game/BP_MapVoteController.VoteEnded` (`self.BP_MapVoteController`) (delegate `OnVoteEnded`)))

(event `Multicast-RoundEnd`
  (params (Reason :type String))
  (`self.RoundEnded` Reason))

(event `OnVoteEnded`
  (params (VotedMap :type Name))
  (bind _returnvalue (`|GetDataTableRow` "/Game/Data/DataTables/DT_VoteMaps.DT_VoteMaps" VotedMap)
    (:`then`
      (`self.TravelServerToMap` (break `/Game/Data/Structs/ST_MapInfo` _returnvalue)))))

(event `self.ReceiveBeginPlay`
  (`/Engine/EditorBlueprintResources/ActorMacros.Switch Has Authority`
    (:`Authority`
      (add `/Game/Blueprints/Game/BP_BaseGameMode.RoundEnded` (`/Game/Blueprints/Libs/Functions/BP_Functions_GlobalGetters.GetGameMode`) (delegate `OnRoundEnded`)))))

(event `self.ReceiveTick`
  (params (DeltaSeconds :type "Float (single-precision)"))
  (`/Engine/EditorBlueprintResources/ActorMacros.Switch Has Authority`
    (:`Authority`
      (switch `/Game/Data/Enums/E_GameState` (`self.RoundInProgress`)
        (:`NewEnumerator0`
          (if (`self.EnoughPlayersToStartRound`)
            (bind _result (`/Engine/EditorBlueprintResources/StandardMacros.DecrementInt` (`self.RoundStartTime`))
              (:`  `
                (if (<= _result 0)
                  (`/Game/Blueprints/Game/BP_BaseGameMode.StartRound` (`/Game/Blueprints/Libs/Functions/BP_Functions_GlobalGetters.GetGameMode`))
                  (set `self.RoundInProgress` "NewEnumerator1"))))
            (else
              (set `self.RoundStartTime` (defaults `/Game/Blueprints/Game/BP_BaseGameState` (`GameplayStatics.GetObjectClass` self))))))
        (:`NewEnumerator1`
          (`self.RoundTimeTick`))))))

(fn `EnoughPlayersToStartRound`
  (returns (Out :type Boolean))
  (return (>= (`KismetArrayLibrary.Array_Length` (`self.PlayerArray`)) (`self.PlayersNeedToStart`))))

(fn `GetPreRoundTime`
  (returns (Seconds :type Integer))
  (return (`self.RoundStartTime`)))

(fn `GetRoundTime`
  (returns (Minutes :type Integer) (Seconds :type Integer))
  (return (`self.CurrentMinute`) (`self.CurrentSecond`)))

(fn `NewPlayerConnected`
  (params (PlayerState :type "/Game/Blueprints/Player/BP_PlayerState Object Reference"))
  (`KismetSystemLibrary.PrintString` (`KismetStringLibrary.Concat_StrStr` (`KismetSystemLibrary.GetDisplayName` PlayerState) " connected") false)
  (`self.PlayerConnected` PlayerState))

(fn `OnRep_RoundInProgress`
  (switch `/Game/Data/Enums/E_GameState` (`self.RoundInProgress`)
    (:`NewEnumerator1`
      (`self.RoundStarted`))))

(fn `RoundTimeTick`
  (bind _output_get (set `self.RoundTime` (+ (`self.RoundTime`) (`KismetMathLibrary.MakeTimespan` 0 0 0 1)))) ; +1 sec to round time
  (bind (_days _hours _minutes _seconds) (`KismetMathLibrary.BreakTimespan` _output_get))
  (set `self.CurrentSecond` _seconds)
  (set `self.CurrentMinute` _minutes)
  (if (and (>= (`self.RoundTime`) (`/Game/Blueprints/Game/BP_BaseGameMode.TimeLimit` (`/Game/Blueprints/Libs/Functions/BP_Functions_GlobalGetters.GetGameMode`))) (`|EnumEquality` (`self.RoundInProgress`) "NewEnumerator1"))
    (`/Game/Blueprints/Game/BP_BaseGameMode.TimeLimitReached` (`/Game/Blueprints/Libs/Functions/BP_Functions_GlobalGetters.GetGameMode`))))

(fn `TravelServerToMap`
  (params (Map :type Name))
  (`KismetSystemLibrary.ExecuteConsoleCommand` (`KismetStringLibrary.Concat_StrStr` "ServerTravel " (`KismetStringLibrary.Conv_NameToString` Map))))

(fn `UserConstructionScript`)