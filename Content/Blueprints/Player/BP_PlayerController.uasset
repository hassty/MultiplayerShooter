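; Player controller that handles respawning, HUD menu input, chat and map voting.
; Enter while spectating requests a server respawn if the game mode allows fast respawn; a timed respawn clears when the round ends, and both spawn through the game mode.
; Tab and chat keys toggle HUD panels, while server events pass messages and votes to game state controllers.
; A spectator spawn function, tagged REMOVE, possesses a follow or free spectator.
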(event `self.ReceiveBeginPlay`
  (`/Engine/EditorBlueprintResources/StandardMacros.IsValid` (`self.GetOwner`)
    (:`Is Valid`
      (`WidgetBlueprintLibrary.SetInputMode_GameOnly` null))))

(event `Key|Enter`
  (params (Key :type "Key Structure"))
  ;[1 1 1] Fast respawn
  (:`Pressed`
    (cast `/Game/Blueprints/Game/Spectators/BP_GameSpectator` (`self.K2_GetPawn`))
    (`self.Server-Respawn`)))

(event `RoundEndedInRespawn`
  (params (Reason :type String))
  (remove `/Game/Blueprints/Game/BP_BaseGameMode.RoundEnded` (`/Game/Blueprints/Libs/Functions/BP_Functions_GlobalGetters.GetGameMode`) (delegate `RoundEndedInRespawn`))
  (`KismetSystemLibrary.K2_ClearAndInvalidateTimerHandle` (`self.RespawnTimer`)))

(event `Server-Respawn`
  ;[1 1 1] Fast respawn
  (bind _asbp_base_game_mode (cast `/Game/Blueprints/Game/BP_BaseGameMode` (`GameplayStatics.GetGameMode`)))
  (if (`/Game/Blueprints/Game/BP_BaseGameMode.AllowFastRespawn` _asbp_base_game_mode)
    (`self.Respawn`)))

(event `Key|Tab`
  (params (Key :type "Key Structure"))
  (bind _hud (`/Game/Blueprints/Libs/Functions/BP_Functions_GlobalGetters.GetPlayerHUD`))
  ;[1 1 1] Tab menu
  (:`Pressed`
    (`/Game/Blueprints/Game/BP_BaseHUD.ToggleTab` _hud true)
    (`/Game/Blueprints/Game/BP_BaseHUD.ToggleHUD` _hud false))
  (:`Released`
    (`/Game/Blueprints/Game/BP_BaseHUD.ToggleTab` _hud false)
    (`/Game/Blueprints/Game/BP_BaseHUD.ToggleHUD` _hud true)))

(event `SendChatMessageToServer`
  (params (Message :type Text))
  (`/Game/Blueprints/Components/Game/BP_ChatController.PostMessage` (`/Game/Blueprints/Game/BP_BaseGameState.BP_ChatController` (`/Game/Blueprints/Libs/Functions/BP_Functions_GlobalGetters.GetGameState`)) Message (cast `/Game/Blueprints/Player/BP_PlayerState` (`self.PlayerState`) :!pure true)))

(event `InputAction|ActivateChat`
  (params (Key :type "Key Structure"))
  (:`Pressed`
    (`/Game/Blueprints/Game/BP_BaseHUD.ToggleChat` (`/Game/Blueprints/Libs/Functions/BP_Functions_GlobalGetters.GetPlayerHUD`) true)))

(event `Key|Escape`
  (params (Key :type "Key Structure"))
  (bind _hud (`/Game/Blueprints/Libs/Functions/BP_Functions_GlobalGetters.GetPlayerHUD`))
  (:`Pressed`
    (if (`/Game/Blueprints/Game/BP_BaseHUD.IsChatActive` _hud)
      (`/Game/Blueprints/Game/BP_BaseHUD.ToggleChat` _hud false))))

(event `SendVoteToServer`
  (params (MapIndex :type Integer))
  (`/Game/Blueprints/Components/Game/BP_MapVoteController.SetVote` (`/Game/Blueprints/Game/BP_BaseGameState.BP_MapVoteController` (`/Game/Blueprints/Libs/Functions/BP_Functions_GlobalGetters.GetGameState`)) MapIndex (cast `/Game/Blueprints/Player/BP_PlayerState` (`self.PlayerState`) :!pure true)))

(fn `CharacterPossess`
  (params (Char :type "/Game/Blueprints/Player/BP_PlayerCharacter Object Reference"))
  (`self.PossessedToChar` Char))

(fn `LaunchRespawnTimer`
  (params (Time :type "Float (double-precision)"))
  (bind _returnvalue (`KismetSystemLibrary.K2_SetTimer` null "Respawn" Time))
  (set `self.RespawnTimer` _returnvalue)
  (add `/Game/Blueprints/Game/BP_BaseGameMode.RoundEnded` (`/Game/Blueprints/Libs/Functions/BP_Functions_GlobalGetters.GetGameMode`) (`|CreateDelegate` :!event `RoundEndedInRespawn`)))

(fn `Respawn`
  (bind _asbp_base_game_mode (cast `/Game/Blueprints/Game/BP_BaseGameMode` (`GameplayStatics.GetGameMode`)))
  (`/Game/Blueprints/Game/BP_BaseGameMode.SpawnPlayer` _asbp_base_game_mode self))

(fn `SpawnAsSpectatorREMOVE`
  (params (DeathInstigatorChar :type "/Game/Blueprints/Player/BP_PlayerCharacter Object Reference"))
  (locals (L_Instigator :type "/Game/Blueprints/Player/BP_PlayerCharacter Object Reference") (L_Spectator :type "/Game/Blueprints/Game/Spectators/BP_GameSpectator Object Reference"))
  (bind _output_get (set `local.L_Instigator` DeathInstigatorChar))
  (`/Engine/EditorBlueprintResources/StandardMacros.IsValid` _output_get
    (:`Is Valid`
      (bind _returnvalue (`|SpawnActorFromClass` "/Game/Blueprints/Game/Spectators/BP_GameSpectator_CharFollow.BP_GameSpectator_CharFollow_C" (`self.GetTransform` (`local.L_Instigator`)) "Undefined" "OverrideRootScale" null self null))
      (set `local.L_Spectator` _returnvalue))
    (:`Is Not Valid`
      (bind _returnvalue_2 (`|SpawnActorFromClass` "/Game/Blueprints/Game/Spectators/BP_GameSpectator_Free.BP_GameSpectator_Free_C" (`self.GetTransform` (`self.K2_GetPawn`)) "Undefined" "OverrideRootScale" null self null))
      (set `local.L_Spectator` _returnvalue_2)))
  (`self.Possess` (`local.L_Spectator`))
  (bind _asbp_game_spectator_char_follow (cast `/Game/Blueprints/Game/Spectators/BP_GameSpectator_CharFollow` (`local.L_Spectator`)))
  (`/Game/Blueprints/Game/Spectators/BP_GameSpectator_CharFollow.SetFollowCharacter` _asbp_game_spectator_char_follow (`local.L_Instigator`)))

(fn `UserConstructionScript`)